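; Projectile Actor that flies along its local X axis and destroys itself when it overlaps any other actor.
; Each Tick it offsets itself by its relative speed plus the BP_Player pawn's current ForwardSpeed, scaled by delta time, so its speed tracks the player's.
; Movement stops if player pawn 0 is not a BP_Player.
; BeginPlay records a StartTime, which these graphs never read.
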(event `self.ReceiveBeginPlay`
  (set `self.StartTime` (`GameplayStatics.GetTimeSeconds`)))

(event `self.ReceiveActorBeginOverlap`
  (params (OtherActor :type "Actor Object Reference"))
  (`self.K2_DestroyActor`))

(event `self.ReceiveTick`
  (params (DeltaSeconds :type "Float (single-precision)"))
  (bind _asbp_player (cast `/Game/InfiniteMatrix/Blueprints/BP_Player` (`GameplayStatics.GetPlayerPawn` 0)))
  (`self.K2_AddActorLocalOffset` (`KismetMathLibrary.MakeVector` (* DeltaSeconds (+ (`self.ProjectileRelativeSpeed`) (`/Game/InfiniteMatrix/Blueprints/BP_Player.ForwardSpeed` _asbp_player))))))

(fn `UserConstructionScript`)